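; Behavior tree task that picks a random wander destination for a monster AI.
; It sets the MonsterCharacter to walk speed, then looks for a random reachable navigation point within WanderRadius of the pawn.
; On success it writes a point to the PatrolLocation blackboard key, from a second evaluation of the query rather than the one checked.
; It finishes as failed if the cast or search fails.
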(event `self.ReceiveExecuteAI`
  (params (OwnerController :type "AIController Object Reference") (ControlledPawn :type "Pawn Object Reference"))
  (bind (_randomlocation _returnvalue) (`NavigationSystemV1.K2_GetRandomReachablePointInRadius` (`Actor.K2_GetActorLocation` ControlledPawn) (`self.Wander Radius`) null null))
  (bind _asmonster_character (cast `/Game/Blueprints/MonsterCharacter` ControlledPawn)
    (:`then`
      (`/Game/Blueprints/MonsterCharacter.Set Speed` _asmonster_character (`self.Walk Speed`))
      (if _returnvalue
        (`BTFunctionLibrary.SetBlackboardValueAsVector` (`self.PatrolLocation`) _randomlocation)
        (`self.FinishExecute` true)
        (else
          (`self.FinishExecute` false :!label _label))))
    (:`CastFailed`
      (goto _label))))