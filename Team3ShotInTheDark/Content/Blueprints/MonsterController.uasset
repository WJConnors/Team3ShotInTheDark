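; MonsterController is an AI controller for a monster that tracks the player through perception.
; On possess it runs MonsterBehaviourTree.
; Each perception update sets the HasLineOfSight blackboard flag to whether the actor is a successfully sensed Player-tagged actor, and stores that actor as EnemyActor when true.
; EnemyActor is never cleared here, and updates from non-player actors also reset HasLineOfSight to false.
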(event `self.ReceivePossess`
  (params (PossessedPawn :type "Pawn Object Reference"))
  (`self.RunBehaviorTree` "/Game/Blueprints/MonsterBehaviourTree.MonsterBehaviourTree"))

(event `self.AIPerception.OnTargetPerceptionUpdated`
  (params (Actor :type "Actor Object Reference") (Stimulus :type "AIStimulus Structure"))
  (bind _returnvalue (`AIBlueprintHelperLibrary.GetBlackboard` null))
  (bind _returnvalue_2 (and (`self.ActorHasTag` Actor "Player") (`.bSuccessfullySensed` (break `AIStimulus` Stimulus))))
  (`BlackboardComponent.SetValueAsBool` _returnvalue (`self.Has Line of Sight`) _returnvalue_2)
  (if _returnvalue_2
    (`BlackboardComponent.SetValueAsObject` _returnvalue (`self.Enemy Actor`) Actor)))

(fn `UserConstructionScript`)